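; BP_PhotoSphere is a sky sphere that displays 360° panorama photos of the rooms of an interior, such as lounge, bedrooms and office.
; The construction script creates a dynamic instance of a panning sky material on the SkySphere mesh.
; OnSkyboxChangeTexture stores the requested room, then swaps that instance's PanoPhoto texture and sets the same Image_Direction vector for every room.
; BeginPlay caches the controlled PhotoSphere character.
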(event Custom|OnSkyboxChangeTexture
  (params (Room :type E_PhotoSphere_Rooms%20Enum :default "NewEnumerator0"))
  (bind _dynamicmaterial_instance (Variables|Default|GetDynamicMaterial_Instance))
  ;[0 0 0] Change SkySphere Texture
  (bind _output_get (Variables|Default|SetCurrentRoom Room))
  (switch Utilities|FlowControl|Switch|SwitchonE_PhotoSphere_Rooms _output_get
    (:NewEnumerator0
      (Rendering|Material|SetTextureParameterValue _dynamicmaterial_instance "PanoPhoto" "/Game/VRAssets/PhotoSphere/NewB4/T_B4_0_low_compressed.T_B4_0_low_compressed")
      (Rendering|Material|SetVectorParameterValue _dynamicmaterial_instance "Image_Direction" (Utilities|Struct|MakeLinearColor -1.0 -1.0 -1.0 1.0) :!class /Script/Engine.MaterialInstanceDynamic))
    (:NewEnumerator1
      (Rendering|Material|SetTextureParameterValue _dynamicmaterial_instance "PanoPhoto" "/Game/VRAssets/PhotoSphere/NewB4/T_B4_1_low_compressed.T_B4_1_low_compressed")
      (Rendering|Material|SetVectorParameterValue _dynamicmaterial_instance "Image_Direction" (Utilities|Struct|MakeLinearColor -1.0 -1.0 -1.0 1.0) :!class /Script/Engine.MaterialInstanceDynamic))
    (:NewEnumerator2
      (Rendering|Material|SetTextureParameterValue _dynamicmaterial_instance "PanoPhoto" "/Game/VRAssets/PhotoSphere/NewB4/T_B4_2_low_compressed.T_B4_2_low_compressed")
      (Rendering|Material|SetVectorParameterValue _dynamicmaterial_instance "Image_Direction" (Utilities|Struct|MakeLinearColor -1.0 -1.0 -1.0 1.0) :!class /Script/Engine.MaterialInstanceDynamic))
    (:NewEnumerator3
      (Rendering|Material|SetTextureParameterValue _dynamicmaterial_instance "PanoPhoto" "/Game/VRAssets/PhotoSphere/NewB4/T_B4_3_low_compressed.T_B4_3_low_compressed")
      (Rendering|Material|SetVectorParameterValue _dynamicmaterial_instance "Image_Direction" (Utilities|Struct|MakeLinearColor -1.0 -1.0 -1.0 1.0) :!class /Script/Engine.MaterialInstanceDynamic))
    (:NewEnumerator4
      (Rendering|Material|SetTextureParameterValue _dynamicmaterial_instance "PanoPhoto" "/Game/VRAssets/PhotoSphere/NewB4/T_B4_4_low_compressed.T_B4_4_low_compressed")
      (Rendering|Material|SetVectorParameterValue _dynamicmaterial_instance "Image_Direction" (Utilities|Struct|MakeLinearColor -1.0 -1.0 -1.0 1.0) :!class /Script/Engine.MaterialInstanceDynamic))
    (:NewEnumerator5
      (Rendering|Material|SetTextureParameterValue _dynamicmaterial_instance "PanoPhoto" "/Game/VRAssets/PhotoSphere/NewB4/T_B4_5_low_compressed.T_B4_5_low_compressed")
      (Rendering|Material|SetVectorParameterValue _dynamicmaterial_instance "Image_Direction" (Utilities|Struct|MakeLinearColor -1.0 -1.0 -1.0 1.0) :!class /Script/Engine.MaterialInstanceDynamic))
    (:NewEnumerator6
      (Rendering|Material|SetTextureParameterValue _dynamicmaterial_instance "PanoPhoto" "/Game/VRAssets/PhotoSphere/NewB4/T_B4_6_low_compressed.T_B4_6_low_compressed")
      (Rendering|Material|SetVectorParameterValue _dynamicmaterial_instance "Image_Direction" (Utilities|Struct|MakeLinearColor -1.0 -1.0 -1.0 1.0) :!class /Script/Engine.MaterialInstanceDynamic))
    (:NewEnumerator7
      (Rendering|Material|SetTextureParameterValue _dynamicmaterial_instance "PanoPhoto" "/Game/VRAssets/PhotoSphere/NewB4/T_B4_7_low_compressed.T_B4_7_low_compressed")
      (Rendering|Material|SetVectorParameterValue _dynamicmaterial_instance "Image_Direction" (Utilities|Struct|MakeLinearColor -1.0 -1.0 -1.0 1.0) :!class /Script/Engine.MaterialInstanceDynamic))
    (:NewEnumerator8
      (Rendering|Material|SetTextureParameterValue _dynamicmaterial_instance "PanoPhoto" "/Game/VRAssets/PhotoSphere/NewB4/T_B4_8_low_compressed.T_B4_8_low_compressed")
      (Rendering|Material|SetVectorParameterValue _dynamicmaterial_instance "Image_Direction" (Utilities|Struct|MakeLinearColor -1.0 -1.0 -1.0 1.0) :!class /Script/Engine.MaterialInstanceDynamic))))

(event EventBeginPlay
  ;[0 0 0] Init - Set Character
  (bind _asbp_photo_sphere_character (Utilities|Casting|CastToBP_PhotoSphere_Character (Pawn|GetControlledPawn (Game|GetPlayerController 0))))
  (Variables|Default|SetPhotoSphereCharacter _asbp_photo_sphere_character))

(event Collision|EventActorBeginOverlap
  (params (OtherActor :type Actor%20Object%20Reference)))

(event EventTick
  (params (DeltaSeconds :type Float%20%28single-precision%29)))

(fn ConstructionScript
  (bind _returnvalue (Rendering|Material|CreateDynamicMaterialInstance (Variables|Default|GetSkySphere) 0 "/Game/VRAssets/PhotoSphere/M_Sky_Panning_Inst.M_Sky_Panning_Inst" "None" :!class /Script/Engine.PrimitiveComponent))
  (Variables|Default|SetDynamicMaterial_Instance _returnvalue))