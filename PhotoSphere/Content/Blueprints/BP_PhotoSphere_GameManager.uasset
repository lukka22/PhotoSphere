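; Game manager actor, named for the PhotoSphere mode, that controls looping background music according to the player's music setting.
; On BeginPlay it spawns the casual theme as a 2D sound, keeps a reference, then pauses or unpauses it based on IsMusicOn from PMM_GameInstance.
; OnMusicSettingsChanged repeats that check, toggling pause on the existing sound instead of respawning it.
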(event Custom|OnMusicSettingsChanged
  (bind _backgroundmusic (Variables|Default|GetBackgroundMusic))
  ;[0 0 0] Handle music
  (bind _aspmm_game_instance (Utilities|Casting|CastToPMM_GameInstance (Game|GetGameInstance)))
  (bind _ison (Default|IsMusicon _aspmm_game_instance))
  (if _ison
    (Class|AudioComponent|SetPaused _backgroundmusic false)
    (else
      (Class|AudioComponent|SetPaused _backgroundmusic true))))

(event EventBeginPlay
  ;[0 0 0] Init sound
  (bind _returnvalue (Audio|SpawnSound2D "/Game/MegaGameMusicCollection/CasualGameMusicPack/Cues/Casual_Theme__1__Looped__Cue.Casual_Theme__1__Looped__Cue" 1.0 1.0 0.0 0))
  (Variables|Default|SetBackgroundMusic _returnvalue)
  (bind _aspmm_game_instance (Utilities|Casting|CastToPMM_GameInstance (Game|GetGameInstance)))
  (bind _ison (Default|IsMusicon _aspmm_game_instance))
  (if _ison
    (Class|AudioComponent|SetPaused (Variables|Default|GetBackgroundMusic) false)
    (else
      (Class|AudioComponent|SetPaused (Variables|Default|GetBackgroundMusic) true))))

(event Collision|EventActorBeginOverlap
  (params (OtherActor :type Actor%20Object%20Reference)))

(event EventTick
  (params (DeltaSeconds :type Float%20%28single-precision%29)))

(fn ConstructionScript)