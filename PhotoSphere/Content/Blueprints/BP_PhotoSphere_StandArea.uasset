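; BP_PhotoSphere_StandArea is a room stand area in a photo sphere tour that manages the bubble markers shown while the player is in that room.
; Unless hidden, BeginPlay spawns a bubble per Nodes entry, attaches it to RootPopup and passes it room and pointer height.
; Show/hide events toggle bubble widgets, showing them only when the character's CurrentRoomLocation matches RoomName.
; The construction script labels the actor with its room name.
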(event Custom|OnWidgetsNeedtoShow
  ;[0 0 0] Set widget visibility when needed
  (if (not (Variables|Default|GetIsHidden))
    (CallFunction|OnWidgetsNeedtoHide)
    (bind _isplayerhere (CallFunction|IsPlayerHere))
    (if _isplayerhere
      (for _array_element (Variables|Default|GetWidgetNodes)
        (Rendering|SetVisibility (Variables|/Game/Blueprints/BP_PhotoSphere_StandArea_Bubble.BP_PhotoSphere_StandArea_Bubble_C|GetWidget _array_element) true false)))))

(event Custom|OnWidgetsNeedtoHide
  ;[0 0 0] Set widget visibility when needed
  (if (not (Variables|Default|GetIsHidden))
    (for _array_element (Variables|Default|GetWidgetNodes)
      (Rendering|SetVisibility (Variables|/Game/Blueprints/BP_PhotoSphere_StandArea_Bubble.BP_PhotoSphere_StandArea_Bubble_C|GetWidget _array_element) false false))))

(event EventBeginPlay
  ;[0 0 0] init - bubble node list and set the visibility option
  (if (not (Variables|Default|GetIsHidden))
    (for _array_element (Variables|Default|GetNodes) ; loop through listed nodes
      (bind _returnvalue (Game|SpawnActorfromClass "/Game/Blueprints/BP_PhotoSphere_StandArea_Bubble.BP_PhotoSphere_StandArea_Bubble_C" (Math|Transform|MakeTransform (.location _array_element) "0, 0, 0" "1,1,1") "AlwaysSpawn" self 0))
      (Transformation|AttachComponentToComponent (Variables|/Script/Engine.Actor|GetRootComponent _returnvalue) (Variables|Default|GetRootPopup) "None" "KeepWorld" "KeepWorld" "KeepWorld" true)
      (Variables|/Game/Blueprints/BP_PhotoSphere_StandArea_Bubble.BP_PhotoSphere_StandArea_Bubble_C|SetParentActor _returnvalue self)
      (Variables|/Game/Blueprints/BP_PhotoSphere_StandArea_Bubble.BP_PhotoSphere_StandArea_Bubble_C|SetRoomName _returnvalue (.room _array_element))
      (Variables|/Game/Blueprints/BP_PhotoSphere_StandArea_Bubble.BP_PhotoSphere_StandArea_Bubble_C|SetPointerHeight _returnvalue (.pointerheight _array_element))
      (Utilities|Array|Add (Variables|Default|GetWidgetNodes) _returnvalue)
      (Default|OnPhotoSphereBubbleReadytoInit _returnvalue)
      (bind _isplayerhere (CallFunction|IsPlayerHere))
      (if _isplayerhere
        (for _array_element_2 (Variables|Default|GetWidgetNodes)
          (Rendering|SetVisibility (Variables|/Game/Blueprints/BP_PhotoSphere_StandArea_Bubble.BP_PhotoSphere_StandArea_Bubble_C|GetWidget _array_element_2) true false))
        (else
          (for _array_element_3 (Variables|Default|GetWidgetNodes)
            (Rendering|SetVisibility (Variables|/Game/Blueprints/BP_PhotoSphere_StandArea_Bubble.BP_PhotoSphere_StandArea_Bubble_C|GetWidget _array_element_3) false false)))))))

(event Collision|EventActorBeginOverlap
  (params (OtherActor :type Actor%20Object%20Reference)))

(fn ConstructionScript
  (Rendering|Components|TextRender|SetText (Variables|Default|GetTextRender) (Utilities|Text|ToText(String) (Utilities|String|EnumtoString (Variables|Default|GetRoomName)))))

(fn IsPlayerHere
  (bind _asbp_photo_sphere_character (Utilities|Casting|CastToBP_PhotoSphere_Character (Game|GetPlayerCharacter 0)))
  (return (Utilities|Enum|Equal(Enum) (Variables|/Game/PhotoSphere/Blueprint/BP_PhotoSphere_Character.BP_PhotoSphere_Character_C|GetCurrentRoomLocation _asbp_photo_sphere_character) (Variables|Default|GetRoomName))))