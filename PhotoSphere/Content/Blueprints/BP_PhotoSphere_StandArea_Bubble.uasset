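; Point-of-interest bubble actor that shows a WB_PointIcon widget linked to a photo sphere room's stand area.
; When ready to init, it finds the BP_PhotoSphere_StandArea with a matching RoomName and passes its player spawn location to the icon as the target point.
; It also hands the icon the room name and pointer height.
; A Tick routine for smoothly rotating the bubble toward the player camera is disconnected and never runs.
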(event Custom|OnPhotoSphereBubble_ReadyToInit
  ;[0 0 0] On setting up point of interest
  (bind _aswb_point_icon (Utilities|Casting|CastToWB_PointIcon (UserInterface|GetUserWidgetObject (Variables|Default|GetWidget))))
  (bind _outactors (Actor|GetAllActorsOfClass "/Game/Blueprints/BP_PhotoSphere_StandArea.BP_PhotoSphere_StandArea_C"))
  (for _array_element _outactors
    (if (Utilities|Enum|Equal(Enum) (Variables|/Game/Blueprints/BP_PhotoSphere_StandArea.BP_PhotoSphere_StandArea_C|GetRoomName _array_element) (Variables|Default|GetRoomName))
      (Variables|/Game/3DMenus/WB_PointIcon.WB_PointIcon_C|SetTargetPointLocation _aswb_point_icon (Transformation|GetWorldLocation (Variables|/Game/Blueprints/BP_PhotoSphere_StandArea.BP_PhotoSphere_StandArea_C|GetRootPlayerSpawn _array_element)))))
  (Variables|/Game/3DMenus/WB_PointIcon.WB_PointIcon_C|SetRoom _aswb_point_icon (Variables|Default|GetRoomName))
  (Variables|/Game/3DMenus/WB_PointIcon.WB_PointIcon_C|SetPointerHeight _aswb_point_icon (Variables|Default|GetPointerHeight)))

(event EventTick
  (params (DeltaSeconds :type Float%20%28single-precision%29))
  ;[1 0 0] DISABLED Make the object rotate to face Player
)

(fn ConstructionScript)