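; Bubble marker for a photo sphere stand area, showing a WB_PointIcon widget that identifies a room and a target point.
; On OnPhotoSphereBubble_ReadyToInit, it passes its RoomName and the RootPlayerSpawn location of its parent BP_PhotoSphere_StandArea to the widget.
; An interpolated face-the-camera rotation is left disconnected from Tick, noted as disabled for screen-space use.
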(event Custom|OnPhotoSphereBubble_ReadyToInit
  (bind _aswb_point_icon (Utilities|Casting|CastToWB_PointIcon (UserInterface|GetUserWidgetObject (Variables|Default|GetWidget)))
    (:then
      (bind _asbp_photo_sphere_stand_area (Utilities|Casting|CastToBP_PhotoSphere_StandArea (Variables|Default|GetParentActor))))
    (:CastFailed
      _))
  (Variables|/Game/3DMenus/WB_PointIcon.WB_PointIcon_C|SetRoom _aswb_point_icon (Variables|Default|GetRoomName))
  (Variables|/Game/3DMenus/WB_PointIcon.WB_PointIcon_C|SetTargetPointLocation _aswb_point_icon (Transformation|GetWorldLocation (Variables|/Game/Blueprints/BP_PhotoSphere_StandArea.BP_PhotoSphere_StandArea_C|GetRootPlayerSpawn _asbp_photo_sphere_stand_area))))

(event EventBeginPlay)

(event Collision|EventActorBeginOverlap
  (params (OtherActor :type Actor%20Object%20Reference)))

(event EventTick
  (params (DeltaSeconds :type Float%20%28single-precision%29))
  ;[1 0 0] DISABLED if using screen spaceRotating to face Player
)

(fn ConstructionScript)