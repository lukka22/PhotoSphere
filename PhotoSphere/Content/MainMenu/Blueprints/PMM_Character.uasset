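; Main menu character that turns touch input into camera rotation, swipes, taps and pinch zoom, and reports touch state to the HUD's main menu widget.
; Release classifies swipes by distance and dominant axis, or taps by a short click-count delay, with double tap zooming out.
; Single-finger drags add controller yaw and pitch, with first-finger drags also feeding the menu's horizontal scroll value.
; Two-finger pinches compare current finger spread against the spread at press to zoom.
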(event EventBeginPlay
  ;[0 0 0] Init Char
  (|CallParentFunction)
  (bind _aspmm_hud (Utilities|Casting|CastToPMM_HUD (HUD|GetHUD (Game|GetPlayerController 0))))
  (Variables|Default|SetMainMenu_Instance (Variables|/Game/MainMenu/Blueprints/PMM_HUD.PMM_HUD_C|GetWB_MainMenu _aspmm_hud)))

(event Collision|EventActorBeginOverlap
  (params (OtherActor :type Actor%20Object%20Reference))
  (|CallParentFunction OtherActor) ; This node is disabled and will not be called.\nDrag off pins to build functionality.
)

(event EventTick
  (params (DeltaSeconds :type Float%20%28single-precision%29)))

(event Input|TouchEvents|InputTouch
  (params (Location :type Vector) (FingerIndex :type ETouchIndex%20Enum))
  (bind _returnvalue (Utilities|Time|GetWorldDeltaSeconds))
  (bind _touch_turnspeed (Variables|Default|GetTouch_TurnSpeed))
  ;[0 0 0] Touch Control mechanism
  (:Pressed
    (bind _mainmenu (CallFunction|GetMainMenu))
    (Variables|/Game/MainMenu/UI/WB_MainMenu.WB_MainMenu_C|SetTouch_isTouching _mainmenu true)
    (bind _output_get (Variables|Default|SetFingerIndex FingerIndex))
    (bind (_touchlocation _touchindexoutput) (CallFunction|GetMouseMovement _output_get))
    (bind _touchend (CallFunction|GetTouchStartEndValue _touchindexoutput))
    (CallFunction|SetTouchStartEndValue _touchlocation _touchend _touchindexoutput)
    (Variables|Default|SetStartLocation _touchlocation)
    (bind _touchlocation_2 (CallFunction|GetMouseMovement "Touch1"))
    (bind _touchlocation_3 (CallFunction|GetMouseMovement "Touch2"))
    (Variables|Default|SetPinch_VectorLengthStart (Math|Vector2D|Vector2DLength (- _touchlocation_2 _touchlocation_3)))
    (Development|PrintString "reset start"))
  (:Released
    (bind _mainmenu_2 (CallFunction|GetMainMenu))
    (Variables|/Game/MainMenu/UI/WB_MainMenu.WB_MainMenu_C|SetTouch_isTouching _mainmenu_2 false)
    (bind (_touchlocation_4 _touchindexoutput_2) (CallFunction|GetMouseMovement FingerIndex))
    (if (Utilities|Enum|Equal(Enum) _touchindexoutput_2 "Touch1")
      (CallFunction|OnTouchOneReleased (Variables|Default|GetisTouchTwo))
      (Variables|Default|SetisTouchJustReleased true :!label _label)
      (Variables|Default|SetEndLocation _touchlocation_4)
      (if (> (Math|Vector2D|Vector2DLength (- (Variables|Default|GetStartLocation) (Variables|Default|GetEndLocation))) 3e+01)
        (Variables|Default|SetIsSwipe true) ; SWIPE
        (if (> (Math|Float|Absolute(Float) (.X (Math|Vector2D|BreakVector2D (- (Variables|Default|GetStartLocation) (Variables|Default|GetEndLocation))))) (Math|Float|Absolute(Float) (.Y (Math|Vector2D|BreakVector2D (- (Variables|Default|GetStartLocation) (Variables|Default|GetEndLocation)))))) ; Up/Down or Left/Right
          (if (> (.X (Math|Vector2D|BreakVector2D (- (Variables|Default|GetStartLocation) (Variables|Default|GetEndLocation)))) 0.0) ; Right / Left
            (Variables|Default|SetPreviousAction (Variables|Default|GetTouchAction))
            (Variables|Default|SetTouchAction "NewEnumerator0")
            (Default|CallOnSwipeRight)
            (else
              (Variables|Default|SetPreviousAction (Variables|Default|GetTouchAction))
              (Variables|Default|SetTouchAction "NewEnumerator1")
              (Default|CallOnSwipeLeft)))
          (elif (> (.Y (Math|Vector2D|BreakVector2D (- (Variables|Default|GetStartLocation) (Variables|Default|GetEndLocation)))) 0.0) ; Up/Down
            (Variables|Default|SetPreviousAction (Variables|Default|GetTouchAction))
            (Variables|Default|SetTouchAction "NewEnumerator2")
            (Default|CallOnSwipeUp)
            (else
              (Variables|Default|SetPreviousAction (Variables|Default|GetTouchAction))
              (Variables|Default|SetTouchAction "NewEnumerator3")
              (Default|CallOnSwipeDown))))
        (else
          (Variables|Default|SetIsSwipe false) ; TAP
          (CallFunction|OnTap)
          (Variables|Default|SetClickCount (+ (Variables|Default|GetClickCount) 1))
          (Utilities|FlowControl|Delay 0.2)
          (if (>= (Variables|Default|GetClickCount) 2)
            (Variables|Default|SetClickCount 0)
            (Variables|Default|SetPreviousAction (Variables|Default|GetTouchAction))
            (Variables|Default|SetTouchAction "NewEnumerator5")
            (CallFunction|PinchZoomout)
            (else
              (Variables|Default|SetClickCount 0)
              (Variables|Default|SetPreviousAction (Variables|Default|GetTouchAction))
              (Variables|Default|SetTouchAction "NewEnumerator4")))))
      (elif (Utilities|Enum|Equal(Enum) _touchindexoutput_2 "Touch2") ; ignore touch > 2
        (CallFunction|OnTouchTwoReleased (Variables|Default|GetisTouchOne))
        (goto _label))))
  (:Moved
    (bind (_touchlocation_5 _touchindexoutput_3) (CallFunction|GetMouseMovement FingerIndex))
    (bind _touchstart (CallFunction|GetTouchStartEndValue _touchindexoutput_3))
    (CallFunction|SetTouchStartEndValue _touchstart _touchlocation_5 _touchindexoutput_3)
    (Utilities|FlowControl|Sequence ; 0 : Swipe to rotate; 1 : Pinch to zoom;
      (:then_0
        (if (Variables|Default|GetisSingleTouch)
          (if (Variables|Default|GetisTouchJustReleased)
            (Variables|Default|SetisTouchJustReleased false)
            (elif (Variables|Default|GetisTouchOne)
              (bind (_touchstart_2 _touchend_2) (CallFunction|GetTouchStartEndValue "Touch1"))
              ;;[0 0 0] apply controller pitch and yaw
              (Pawn|Input|AddControllerYawInput (* (.x (- _touchstart_2 _touchend_2)) _returnvalue _touch_turnspeed))
              (Pawn|Input|AddControllerPitchInput (* (.y (- _touchstart_2 _touchend_2)) _returnvalue (Variables|Default|GetTouch_TurnSpeed)))
              (bind _mainmenu_3 (CallFunction|GetMainMenu))
              (Utilities|IsValid _mainmenu_3
                (:Is%20Valid
                  (Variables|/Game/MainMenu/UI/WB_MainMenu.WB_MainMenu_C|SetTouch_HorizontalScrollValue _mainmenu_3 (* (.x (- _touchstart_2 _touchend_2)) _returnvalue _touch_turnspeed)))
                (:Is%20Not%20Valid
                  _))
              (else
                (bind (_touchstart_3 _touchend_3) (CallFunction|GetTouchStartEndValue "Touch2"))
                (Pawn|Input|AddControllerYawInput (* (.x (- _touchstart_3 _touchend_3)) _returnvalue _touch_turnspeed))
                (Pawn|Input|AddControllerPitchInput (* (.y (- _touchstart_3 _touchend_3)) _returnvalue _touch_turnspeed)))))
          (Variables|Default|SetTouchOne_StartLocationOld (Variables|Default|GetTouchOne_StartLocation)) ; TODO : set based on touch index
          (if (Variables|Default|GetisTouchOne)
            (bind (_touchlocation_6 _touchindexoutput_4) (CallFunction|GetMouseMovement "Touch1"))
            (bind _touchend_4 (CallFunction|GetTouchStartEndValue _touchindexoutput_4))
            (CallFunction|SetTouchStartEndValue _touchlocation_6 _touchend_4 _touchindexoutput_4)
            (else
              (bind (_touchlocation_7 _touchindexoutput_5) (CallFunction|GetMouseMovement "Touch2"))
              (bind _touchend_5 (CallFunction|GetTouchStartEndValue _touchindexoutput_5))
              (CallFunction|SetTouchStartEndValue _touchlocation_7 _touchend_5 _touchindexoutput_5)))))
      (:then_1
        (Utilities|FlowControl|Delay 0.001)
        (if (Variables|Default|GetisPinching)
          (bind _touchlocation_8 (CallFunction|GetMouseMovement "Touch1"))
          (bind _touchlocation_9 (CallFunction|GetMouseMovement "Touch2"))
          (bind _output_get_2 (Variables|Default|SetPinch_VectorLengthEnd (Math|Vector2D|Vector2DLength (- _touchlocation_8 _touchlocation_9))))
          (if (> _output_get_2 (Variables|Default|GetPinch_VectorLengthStart))
            (CallFunction|PinchZoomin)
            (else
              (CallFunction|PinchZoomout))))))))

(fn ConstructionScript
  (|CallParentFunction))

(fn GetMainMenu
  (bind _aspmm_hud (Utilities|Casting|CastToPMM_HUD (HUD|GetHUD (Game|GetPlayerController 0))))
  (bind _output_get (Variables|Default|SetMainMenu_Instance (Variables|/Game/MainMenu/Blueprints/PMM_HUD.PMM_HUD_C|GetWB_MainMenu _aspmm_hud)))
  (return _output_get))